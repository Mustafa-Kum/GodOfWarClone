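; BP_HeroCharacter is the player hero character Blueprint, handling a camera angle switch and opening the pause screen.
; ChangeCameraAngle alternates FollowCamera's parent between HeavyAttackCameraAngle and CameraBoom, keeping world transform on attach and then moving it with MoveComponentTo.
; IA_PauseMenu async-loads the WBP_PauseScreen class, then creates the widget and adds it to the viewport, without pausing the game here.
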(event `self.ReceiveBeginPlay`)

(event `ChangeCameraAngle`
  (`/Engine/EditorBlueprintResources/StandardMacros.FlipFlop`
    (:`A`
      (`SceneComponent.K2_AttachToComponent` (`self.FollowCamera`) (`self.HeavyAttackCameraAngle`) "None" "KeepWorld" "KeepWorld" "KeepWorld" true))
    (:`B`
      (`SceneComponent.K2_AttachToComponent` (`self.FollowCamera`) (`self.CameraBoom`) "None" "KeepWorld" "KeepWorld" "KeepWorld" true)))
  (`KismetSystemLibrary.MoveComponentTo` (`self.FollowCamera`)))

(event `EnhancedInput|/Game/PlayerCharacter/Input/Actions/IA_PauseMenu`
  (params (ActionValue :type Boolean) (ElapsedSeconds :type "Float (double-precision)") (TriggeredSeconds :type "Float (double-precision)") (InputAction :type "InputAction Object Reference" :default "/Game/PlayerCharacter/Input/Actions/IA_PauseMenu.IA_PauseMenu"))
  (:`Started`
    (bind _class (`|LoadAssetClass` "/Game/Widgets/GameModeWidgets/WBP_PauseScreen.WBP_PauseScreen_C")
      (:`Completed`
        (bind _asuser_widget (castclass `UserWidget` _class))
        (bind _returnvalue (`|CreateWidget` _asuser_widget))
        (`UserWidget.AddToViewport` _returnvalue 0)))))

(fn `UserConstructionScript`)